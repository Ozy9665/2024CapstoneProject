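; BP_GCSlab is a Chaos slab actor whose GCComp, likely a Geometry Collection, is held static when play starts.
; BeginPlay turns off the component's physics simulation and gravity, then runs a short delay with nothing after it.
; An unconnected chain that would enable blocking collision and print the collision state never runs.
; Overlap, Tick and the construction script are empty.
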(event `self.ReceiveBeginPlay`
  (bind _gccomp (`self.GCComp`))
  (`PrimitiveComponent.SetSimulatePhysics` _gccomp false)
  (`PrimitiveComponent.SetEnableGravity` _gccomp false)
  (`KismetSystemLibrary.Delay` 1.0))

(fn `UserConstructionScript`)