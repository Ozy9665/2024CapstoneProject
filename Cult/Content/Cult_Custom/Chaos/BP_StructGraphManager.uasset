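; BP_StructGraphManager handles staged structural destruction events, from a local break to the ending collapse.
; The Stage 2 break wakes the target geometry collection with physics and gravity, without using its hit, radius or strain inputs.
; Stage 3 start enters cinematic mode and plays the collapse sequence; its end shows the game result widget with UI-only input.
; Node yield and failure handlers are empty, leaving debug, effect and sound nodes unconnected.
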(event `self.OnNodeYield`
  (params (Comp :type "PrimitiveComponent Object Reference") (Utilization :type "Float (single-precision)")))

(event `self.OnNodeFailed`
  (params (Comp :type "PrimitiveComponent Object Reference") (Utilization :type "Float (single-precision)")))

(event `Stage2_LocalBreak`
  (params (TargetGC :type "GeometryCollectionComponent Object Reference") (HitLocation :type "Vector Structure") (Radius :type "Float (double-precision)" :default 120.0) (Strain :type "Float (double-precision)" :default 80000.0))
  (if (`KismetSystemLibrary.IsValid` TargetGC)
    (`PrimitiveComponent.SetSimulatePhysics` TargetGC true)
    (`PrimitiveComponent.SetEnableGravity` TargetGC true)
    (`PrimitiveComponent.WakeAllRigidBodies` TargetGC)))

(event `self.BP_OnStage3Started`
  (bind _returnvalue (`GameplayStatics.GetPlayerController` 0))
  (`PlayerController.SetCinematicMode` _returnvalue true true false false false)
  (`PlayerController.SetViewTargetWithBlend` _returnvalue null 1.0 "VTBlend_Linear" 0.0 false)
  (bind (_outactor _returnvalue_2) (`LevelSequencePlayer.CreateLevelSequencePlayer` "/Game/Cult_Custom/Sequence/LS_EndingCollapse.LS_EndingCollapse" (make `MovieSceneSequencePlaybackSettings` false (struct) 1.0 0.0 false true false false false false "ForceKeepState" true)))
  (`MovieSceneSequencePlayer.Play` _returnvalue_2))

(event `self.BP_OnStage3Ended`
  (bind _returnvalue (`|CreateWidget` "/Game/Cult_Custom/WBP_GameResult.WBP_GameResult_C"))
  (`UserWidget.AddToViewport` _returnvalue 0)
  (`WidgetBlueprintLibrary.SetInputMode_UIOnlyEx` (`GameplayStatics.GetPlayerController` 0) null))

(fn `UserConstructionScript`)