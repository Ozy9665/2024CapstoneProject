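; Test rig actor that simulates an earthquake on static mesh slabs with physics impulses and a camera shake.
; BeginPlay caches a static mesh component from each actor carrying the slab tag.
; StartEarthQuake resets state, plays the shake, enables slab physics and sets a looping tick timer plus a stop timer.
; Each tick applies a circular sine/cosine horizontal impulse with upward lift as velocity change, until StopEarthquake clears the loop.
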(event `StartEarthQuake`
  (`KismetSystemLibrary.K2_ClearAndInvalidateTimerHandle` (`self.EarthquakeTimerHandle`))
  (`KismetSystemLibrary.K2_ClearAndInvalidateTimerHandle` (`self.StopTimerHandle`))
  (set `self.Elapsed` 0.0)
  (`PlayerCameraManager.StartCameraShake` :`self` (`PlayerController.PlayerCameraManager` (`GameplayStatics.GetPlayerController` 0)) :`ShakeClass` "/Game/Cult_Custom/Chaos/BP_EQ_LegacyShake.BP_EQ_LegacyShake_C")
  (for _array_element (`self.SlabMeshes`)
    (`PrimitiveComponent.SetSimulatePhysics` _array_element true)
    (`PrimitiveComponent.WakeRigidBody` _array_element "None")
    (bind _returnvalue (`KismetSystemLibrary.K2_SetTimerDelegate` (delegate `ApplyEarthquakeTick`) (`self.TickInterval`) true))
    (set `self.EarthquakeTimerHandle` _returnvalue)
    (bind _returnvalue_2 (`KismetSystemLibrary.K2_SetTimerDelegate` (delegate `StopEarthquake`) (`self.Duration`)))
    (set `self.StopTimerHandle` _returnvalue_2)))

(event `StopEarthquake`
  (`KismetSystemLibrary.K2_ClearAndInvalidateTimerHandle` (`self.EarthquakeTimerHandle`)))

(event `ApplyEarthquakeTick`
  (bind _angle (`self.Angle`))
  (set `self.Elapsed` (+ (`self.Elapsed`) (`self.TickInterval`)))
  (set `self.Angle` (* (* (`self.Elapsed`) (`self.Frequency`)) 6.283185))
  (for _array_element (`self.SlabMeshes`)
    (`PrimitiveComponent.AddImpulse` _array_element (+ (* (`KismetMathLibrary.MakeVector` (`KismetMathLibrary.Sin` _angle) (`KismetMathLibrary.Cos` _angle)) (`self.ImpulseStrength`)) (`KismetMathLibrary.MakeVector` 0.0 0.0 (`self.UpLiftStrength`))) "None" true)))

(event `self.ReceiveBeginPlay`
  (bind _outactors (`GameplayStatics.GetAllActorsWithTag` (`self.SlabTag`)))
  (for _array_element _outactors
    (bind _returnvalue (`self.GetComponentByClass` _array_element "/Script/Engine.StaticMeshComponent"))
    (if (`KismetSystemLibrary.IsValid` _returnvalue)
      (`KismetArrayLibrary.Array_Add` (`self.SlabMeshes`) _returnvalue)))
  (`KismetSystemLibrary.PrintString` (`KismetStringLibrary.Conv_IntToString` (`KismetArrayLibrary.Array_Length` (`self.SlabMeshes`)))))

(fn `UserConstructionScript`)