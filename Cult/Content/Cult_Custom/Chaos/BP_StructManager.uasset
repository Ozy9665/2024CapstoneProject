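; BP_StructManager gathers a building's structural meshes and forwards three quake-stage inputs to a graph manager.
; On BeginPlay it collects tagged slab, column and wall meshes, grouping slabs by floor and saving their transforms.
; It spawns the graph manager and initializes it with those arrays.
; Column and wall collection, transform saving and spawning all sit inside the slab-tag loop, so they repeat per tag.
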(event `InputAction|QuqkeStage1`
  (params (Key :type "Key Structure"))
  (bind _graphmanagerref (`self.GraphManagerRef`))
  (:`Pressed`
    (if (`KismetSystemLibrary.IsValid` _graphmanagerref)
      (`StructGraphManager.TriggerStage1` _graphmanagerref))))

(event `InputAction|QuqkeStage2`
  (params (Key :type "Key Structure"))
  (bind _graphmanagerref (`self.GraphManagerRef`))
  (:`Pressed`
    (if (`KismetSystemLibrary.IsValid` _graphmanagerref)
      (`StructGraphManager.TriggerStage2` _graphmanagerref))))

(event `InputAction|QuqkeStage3`
  (params (Key :type "Key Structure"))
  (bind _graphmanagerref (`self.GraphManagerRef`))
  (:`Pressed`
    (if (`KismetSystemLibrary.IsValid` _graphmanagerref)
      (`StructGraphManager.TriggerStage3` _graphmanagerref))))

(event `self.ReceiveBeginPlay`
  ;[1 1 1] Clear
  (`KismetArrayLibrary.Array_Clear` (`self.SlabMeshes`))
  (`KismetArrayLibrary.Array_Clear` (`self.SlabMeshes_L1`))
  (`KismetArrayLibrary.Array_Clear` (`self.SlabMeshes_L2`))
  (`KismetArrayLibrary.Array_Clear` (`self.SlabMeshes_L3`))
  (`KismetArrayLibrary.Array_Clear` (`self.SlabMeshes_ROOF`))
  (`KismetArrayLibrary.Array_Clear` (`self.WallMeshes`))
  (`KismetArrayLibrary.Array_Clear` (`self.ColumnMeshes`))
  (`BlueprintMapLibrary.Map_Clear` (`self.OriginalTransforms`))
  ;[1 1 1] Collect Slab
  (for _array_element (`self.SlabTags`)
    (bind _outactors (`GameplayStatics.GetAllActorsWithTag` _array_element))
    (for _array_element_2 _outactors
      (bind _returnvalue (`self.GetComponentByClass` _array_element_2 "/Script/Engine.StaticMeshComponent"))
      (if (`KismetSystemLibrary.IsValid` _returnvalue)
        (`KismetArrayLibrary.Array_AddUnique` (`self.SlabMeshes`) _returnvalue)
        (switch `name` _array_element
          (:`SLAB_L1`
            (`KismetArrayLibrary.Array_AddUnique` (`self.SlabMeshes_L1`) _returnvalue))
          (:`SLAB_L2`
            (`KismetArrayLibrary.Array_AddUnique` (`self.SlabMeshes_L2`) _returnvalue))
          (:`SLAB_L3`
            (`KismetArrayLibrary.Array_AddUnique` (`self.SlabMeshes_L3`) _returnvalue))
          (:`SLAB_ROOF`
            (`KismetArrayLibrary.Array_AddUnique` (`self.SlabMeshes_ROOF`) _returnvalue)))))
    ;[1 1 1] Collect Column
    (bind _outactors_2 (`GameplayStatics.GetAllActorsWithTag` (`self.ColumnTags`)))
    (for _array_element_3 _outactors_2
      (bind _returnvalue_2 (`self.GetComponentByClass` _array_element_3 "/Script/Engine.StaticMeshComponent"))
      (if (`KismetSystemLibrary.IsValid` _returnvalue_2)
        (`KismetArrayLibrary.Array_AddUnique` (`self.ColumnMeshes`) _returnvalue_2)))
    ;[1 1 1] Collect Wall
    (bind _outactors_3 (`GameplayStatics.GetAllActorsWithTag` (`self.WallTag`)))
    (for _array_element_4 _outactors_3
      (bind _returnvalue_3 (`self.GetComponentByClass` _array_element_4 "/Script/Engine.StaticMeshComponent"))
      (if (`KismetSystemLibrary.IsValid` _returnvalue_3)
        (`KismetArrayLibrary.Array_AddUnique` (`self.WallMeshes`) _returnvalue_3)))
    ;[1 1 1] Save Original Transform
    (for _array_element_5 (`self.SlabMeshes_L1`)
      (`BlueprintMapLibrary.Map_Add` (`self.OriginalTransforms`) _array_element_5 (`SceneComponent.K2_GetComponentToWorld` _array_element_5)))
    (for _array_element_6 (`self.SlabMeshes_L2`)
      (`BlueprintMapLibrary.Map_Add` (`self.OriginalTransforms`) _array_element_6 (`SceneComponent.K2_GetComponentToWorld` _array_element_6)))
    (for _array_element_7 (`self.SlabMeshes_L3`)
      (`BlueprintMapLibrary.Map_Add` (`self.OriginalTransforms`) _array_element_7 (`SceneComponent.K2_GetComponentToWorld` _array_element_7)))
    (for _array_element_8 (`self.SlabMeshes_ROOF`)
      (`BlueprintMapLibrary.Map_Add` (`self.OriginalTransforms`) _array_element_8 (`SceneComponent.K2_GetComponentToWorld` _array_element_8)))
    ;[1 1 1] BuildGraphInitialize
    (bind _returnvalue_4 (`|SpawnActorFromClass` (`self.GraphManagerClass`) (`self.GetTransform`) "Undefined" "MultiplyWithRoot" null null))
    (bind _output_get (set `self.GraphManagerRef` _returnvalue_4))
    (if (`KismetSystemLibrary.IsValid` _output_get)
      (`StructGraphManager.InitializeFromBP` (`self.GraphManagerRef`) (`self.SlabMeshes_L1`) (`self.SlabMeshes_L2`) (`self.SlabMeshes_L3`) (`self.SlabMeshes_ROOF`) (`self.ColumnMeshes`) (`self.WallMeshes`)))))

(fn `UserConstructionScript`)