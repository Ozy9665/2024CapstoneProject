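; BP_GCLongWall is a destructible long wall built on a Chaos geometry collection component.
; It turns off physics simulation and gravity at BeginPlay.
; The ApplyStage2Strain event applies external cluster strain through a linear radial falloff field centered on a hit point, with caller-supplied radius and magnitude.
; Break and collision events only print debug messages.
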(event `ApplyStage2Strain`
  (params (HitPoint :type "Vector Structure") (Radius :type "Float (double-precision)") (Magnitude :type "Float (double-precision)"))
  (bind _returnvalue (`AddComponent|NODE_AddRadialFalloff-0`))
  (`GeometryCollectionComponent.ApplyPhysicsField` (`self.GCComp`) true "Chaos_ExternalClusterStrain" null (`RadialFalloff.SetRadialFalloff` _returnvalue Magnitude 0.0 1.0 0.0 Radius HitPoint "Field_Falloff_Linear")))

(event `self.ReceiveBeginPlay`
  (`PrimitiveComponent.SetSimulatePhysics` (`self.GCComp`) false)
  (`PrimitiveComponent.SetEnableGravity` (`self.GCComp`) false)
  (`KismetSystemLibrary.Delay` 1.0))

(event `self.GCComp.OnChaosBreakEvent`
  (params (BreakEvent :type "ChaosBreakEvent Structure (by ref)"))
  (`KismetSystemLibrary.PrintString` "LongWallBreak" true true (struct :`G` 0.66 :`B` 1.0 :`A` 1.0) 10.0))

(event `self.GCComp.OnChaosPhysicsCollision`
  (params (CollisionInfo :type "ChaosPhysicsCollisionInfo Structure (by ref)"))
  (`KismetSystemLibrary.PrintString` "LongWallCollision" true true (struct :`G` 0.66 :`B` 1.0 :`A` 1.0) 10.0))

(fn `UserConstructionScript`)