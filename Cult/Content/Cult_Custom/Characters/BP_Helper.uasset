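; BP_Helper is a set of pure math helpers for offsetting positions and flipping surface normals.
; Up and down moves add or subtract along world Z, while forward, back, left and right moves use the axes of a supplied rotation scaled by a distance.
; ReverseNormal turns a normal into an X-axis rotation and takes its delta against a 180-degree rotator, returning a rotator rather than a vector.
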(fn `MoveVectorBackward`
  (params (InVector :type "Vector Structure") (InRotation :type "Rotator Structure") (SubtractValue :type "Float (double-precision)"))
  (returns (ReturnValue :type "Vector Structure"))
  (return (- InVector (* (`KismetMathLibrary.GetForwardVector` InRotation) SubtractValue))))

(fn `MoveVectorDownward`
  (params (InVector :type "Vector Structure") (SubtractValue :type "Float (double-precision)"))
  (returns (ReturnValue :type "Vector Structure"))
  (return (- InVector (`KismetMathLibrary.MakeVector` 0.0 0.0 SubtractValue))))

(fn `MoveVectorForward`
  (params (InVector :type "Vector Structure") (InRotation :type "Rotator Structure") (AddValue :type "Float (double-precision)"))
  (returns (ReturnValue :type "Vector Structure"))
  (return (+ InVector (* (`KismetMathLibrary.GetForwardVector` InRotation) AddValue))))

(fn `MoveVectorLeft`
  (params (InVector :type "Vector Structure") (InRotation :type "Rotator Structure") (MoveValue :type "Float (double-precision)"))
  (returns (ReturnValue :type "Vector Structure"))
  (return (- InVector (* (`KismetMathLibrary.GetRightVector` InRotation) MoveValue))))

(fn `MoveVectorRight`
  (params (InVector :type "Vector Structure") (InRotation :type "Rotator Structure") (MoveValue :type "Float (double-precision)"))
  (returns (ReturnValue :type "Vector Structure"))
  (return (+ InVector (* (`KismetMathLibrary.GetRightVector` InRotation) MoveValue))))

(fn `MoveVectorUpward`
  (params (InVector :type "Vector Structure") (AddValue :type "Float (double-precision)"))
  (returns (ReturnValue :type "Vector Structure"))
  (return (+ InVector (`KismetMathLibrary.MakeVector` 0.0 0.0 AddValue))))

(fn `ReverseNormal`
  (params (InNormal :type "Vector Structure"))
  (returns (ReturnValue :type "Rotator Structure"))
  (return (`KismetMathLibrary.NormalizedDeltaRotator` (`KismetMathLibrary.MakeRotFromX` InNormal) (struct :`Yaw` 180.0))))