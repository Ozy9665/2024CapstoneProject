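; Player police character with over-shoulder pistol/taser aiming, hitscan pistol shots that trigger cultist hit reactions, and AI noise reports when running.
; Jump runs the Parkour graph, which line-traces wall face, height and thickness, then plays a vault montage with collision off and flying movement, skipping tall walls.
; ParkourComponent is initialized with camera and MotionWarping, but its action call is disconnected, along with much older vault and test logic.
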(event `EmitRunNoise`
  (if (> (`KismetMathLibrary.VSize` (`self.GetVelocity`)) 350.0)
    (`AISense_Hearing.ReportNoiseEvent` (`self.K2_GetActorLocation`) 1.0 self 3000.0 "Noise_Run")))

(event `self.ReceiveBeginPlay`
  (`PlayerController.SetViewTargetWithBlend` (`GameplayStatics.GetPlayerController` 0) (`ChildActorComponent.ChildActor` (`self.Camera`)) 0.0 "VTBlend_Linear" 0.0 false)
  (`WidgetBlueprintLibrary.SetInputMode_GameOnly` (`GameplayStatics.GetPlayerController` 0))
  (message `/ParkourSystem/Interfaces/Parkour_Interface.Set Initialize Referrence` (`self.ParkourComponent`) self (`self.SpringArm`) (`self.MotionWarping`) (`self.Camera`))
  (`KismetSystemLibrary.K2_SetTimerDelegate` (`|CreateDelegate` :!event `EmitRunNoise`) 0.5 true))

(event `InputAction|Aim` :consume false
  (params (Key :type "Key Structure"))
  (:`Pressed`
    (if (not (`self.IsPakour`))
      (switch `EWeaponType` (`self.CurrentWeapon`)
        (:`Pistol`
          _)
        (:`Taser`
          _))
      (set `SpringArmComponent.TargetArmLength` 80.0 (`self.SpringArm`))
      (`SceneComponent.K2_AddLocalTransform` (`self.SpringArm`) (`KismetMathLibrary.Conv_VectorToTransform` (0.0 30.0 -30.0)) false false)
      (set `CharacterMovementComponent.bOrientRotationToMovement` false (`self.CharacterMovement`))
      (set `CharacterMovementComponent.bUseControllerDesiredRotation` true (`self.CharacterMovement`))
      (set `self.IsAiming` true)
      (`self.StartAiming`)))
  (:`Released`
    (if (`self.IsAiming`)
      (switch `EWeaponType` (`self.CurrentWeapon`)
        (:`Pistol`
          _)
        (:`Taser`
          _))
      (set `SpringArmComponent.TargetArmLength` 200.0 (`self.SpringArm`))
      (`SceneComponent.K2_AddLocalTransform` (`self.SpringArm`) (`KismetMathLibrary.Conv_VectorToTransform` (0.0 -30.0 30.0)) false false)
      (set `CharacterMovementComponent.bOrientRotationToMovement` true (`self.CharacterMovement`))
      (set `CharacterMovementComponent.bUseControllerDesiredRotation` false (`self.CharacterMovement`))
      (set `self.IsAiming` false)
      (`self.StopAiming`))))

(event `InputAction|SwitchWeapon`
  (params (Key :type "Key Structure")))

(event `InputAction|Sprint`
  (params (Key :type "Key Structure")))

(event `InputAction|Jump`
  (params (Key :type "Key Structure"))
  ;[1 1 1] VaultWithMotionWarp
)

(event `InputAction|Sprint`
  (params (Key :type "Key Structure"))
  ;[1 1 1] Vault
)

(event `InputAction|Jump`
  (params (Key :type "Key Structure"))
  ;[1 1 1] Vault
  (:`Pressed`
    (`self.Parkour`)))

(event `InputAction|SpecialAbility`
  (params (Key :type "Key Structure")))

(event `Key|SpaceBar`
  (params (Key :type "Key Structure"))
  ;[1 1 1] Detect Wall
)

(event `self.ReceiveTick`
  (params (DeltaSeconds :type "Float (single-precision)"))
  (`|ExecutionSequence`
    (:`then_0`
      (set `self.Wall Height2` (.z (- (`self.Wall Height`) (`self.Wall Location`)))))
    (:`then_1`
      (`self.JumpHelperFunction`))))

(event `self.OnShootPistol`
  (params (HitResult :type "HitResult Structure (by ref)"))
  (bind _returnvalue (`self.K2_GetActorLocation`))
  (bind (_outhit _returnvalue_2) (`KismetSystemLibrary.LineTraceSingle` _returnvalue (+ _returnvalue (* (`self.GetActorForwardVector` (`GameplayStatics.GetPlayerCameraManager` 0)) 10000.0)) "TraceTypeQuery1"))
  (if _returnvalue_2
    (bind (_bblockinghit _binitialoverlap _time _distance _location _impactpoint _normal _impactnormal _physmat _hitactor _hitcomponent _hitbonename) (`GameplayStatics.BreakHitResult` _outhit))
    (bind _asbp_cultist_a (cast `/Game/Cult_Custom/Characters/BP_Cultist_A` (`ActorComponent.GetOwner` _hitcomponent)))
    (message `/Game/Cult_Custom/Characters/Interfaces/BPI_Player.BPI_HitReaction` _asbp_cultist_a _hitbonename)))

(event `self.CapsuleComponent.OnComponentHit`
  (params (HitComponent :type "PrimitiveComponent Object Reference") (OtherActor :type "Actor Object Reference") (OtherComp :type "PrimitiveComponent Object Reference") (NormalImpulse :type "Vector Structure") (Hit :type "HitResult Structure (by ref)")))

(fn `Calculate Wall Height`
  (bind _returnvalue (+ (+ (`self.Wall Location`) (* (`KismetMathLibrary.GetForwardVector` (`KismetMathLibrary.MakeRotFromX` (`self.Wall Normal`))) -10.0)) (0.0 0.0 200.0)))
  (bind _outhit (`KismetSystemLibrary.LineTraceSingleForObjects` :`Start` _returnvalue :`End` (- _returnvalue (0.0 0.0 200.0)) :`ObjectTypes` (`self.Object Types`) :`DrawDebugType` (`self.Draw Debug Type`) :`TraceColor` (struct :`G` 1.0 :`B` 0.003697 :`A` 1.0) :`TraceHitColor` (struct :`R` 1.0 :`G` 0.897106 :`A` 1.0)))
  (set `self.Wall Height` (`.Location` (`GameplayStatics.BreakHitResult` _outhit)))
  (return))

(fn `Calculate Wall Thickness`
  (returns (Location :type "Vector Structure") (ReturnValue :type Boolean))
  (bind _returnvalue (+ (+ (`self.Wall Location`) (* (`KismetMathLibrary.GetForwardVector` (`KismetMathLibrary.MakeRotFromX` (`self.Wall Normal`))) -50.0)) (0.0 0.0 200.0)))
  (bind (_outhit _returnvalue_2) (`KismetSystemLibrary.LineTraceSingleForObjects` :`Start` _returnvalue :`End` (- _returnvalue (0.0 0.0 200.0)) :`ObjectTypes` (`self.Object Types`) :`DrawDebugType` (`self.Draw Debug Type`) :`TraceColor` (struct :`G` 1.0 :`B` 0.003697 :`A` 1.0) :`TraceHitColor` (struct :`R` 1.0 :`G` 0.897106 :`A` 1.0)))
  (return (`.Location` (`GameplayStatics.BreakHitResult` _outhit)) _returnvalue_2))

(fn `Disable Input`
  (`CharacterMovementComponent.SetMovementMode` (`self.CharacterMovement`) "MOVE_Flying" 0)
  (`PrimitiveComponent.SetCollisionEnabled` (`self.CapsuleComponent`) "NoCollision"))

(fn `Enable Input`
  (`CharacterMovementComponent.SetMovementMode` (`self.CharacterMovement`) "MOVE_Falling" 0)
  (`PrimitiveComponent.SetCollisionEnabled` (`self.CapsuleComponent`) "QueryAndPhysics"))

(fn `GetCharacterMovement`
  (returns (ReturnValue :type "CharacterMovementComponent Object Reference"))
  (return (`self.CharacterMovement`)))

(fn `GetIsAiming`
  (returns (ReturnValue :type Boolean))
  (return (`self.IsAiming`)))

(fn `GetIsAttacking`
  (returns (ReturnValue :type Boolean))
  (return (`self.bIsAttacking`)))

(fn `GetIsPakour`
  (returns (ReturnValue :type Boolean))
  (return (`self.IsPakour`)))

(fn `GetIsPerforming`
  (returns (ReturnValue :type Boolean))
  (return false))

(fn `GetIsShooting`
  (returns (ReturnValue :type Boolean))
  (return (`self.bIsShooting`)))

(fn `GetMesh`
  (returns (ReturnValue :type "SkeletalMeshComponent Object Reference"))
  (return (`self.Mesh`)))

(fn `GetMontageLength`
  (params (Input :type "AnimMontage Object Reference"))
  (returns (ReturnValue :type "Float (double-precision)"))
  (return (`AnimationAsset.GetPlayLength` Input)))

(fn `GetMotionWarping`
  (returns (ReturnValue :type "MotionWarpingComponent Object Reference"))
  (return (`self.MotionWarping`)))

(fn `GetNearEnoughToPakour`
  (returns (ReturnValue :type Boolean))
  (return (`self.bIsNearEnoughToPakour`)))

(fn `GetPlayerCapsule`
  (returns (ReturnValue :type "CapsuleComponent Object Reference"))
  (return (`self.CapsuleComponent`)))

(fn `GetVaultType`
  (returns (ReturnValue :type Byte))
  (return (`self.CurrentVaultType`)))

(fn `GetWeaponType`
  (returns (ReturnValue :type "EWeaponType Enum"))
  (return (`self.CurrentWeapon`)))

(fn `JumpHelperFunction`
  (bind (_returnvalue_x _returnvalue_y _returnvalue_z) (`KismetMathLibrary.BreakVector` (`self.K2_GetActorLocation`)))
  (if (`self.JumpHelper`)
    (`self.K2_SetActorLocation` (`KismetMathLibrary.MakeVector` _returnvalue_x _returnvalue_y (`KismetMathLibrary.FInterpTo` _returnvalue_z (+ _returnvalue_z (`self.Wall Height2`)) (`GameplayStatics.GetWorldDeltaSeconds`) 4.0)))))

(fn `UserConstructionScript`)