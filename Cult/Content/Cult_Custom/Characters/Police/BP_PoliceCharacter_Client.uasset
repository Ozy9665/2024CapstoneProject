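; Client-side police character Blueprint that calls SetViewTargetWithBlend on the first player controller at BeginPlay.
; Getter functions, likely from an interface, expose movement, mesh, capsule, aiming state and current weapon, while the parkour, attack, shooting and montage queries return empty defaults.
; The fire input is empty, and the parkour, attack, shoulder-aim camera, bullet and pistol montage logic is left disconnected and never runs.
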(event `self.ReceiveBeginPlay`
  (`PlayerController.SetViewTargetWithBlend` (`GameplayStatics.GetPlayerController` 0) null 0.0 "VTBlend_Linear" 0.0 false))

(event `InputAction|Aim`
  (params (Key :type "Key Structure")))

(event `EnhancedInput|/Game/Cult_Custom/Characters/Police/Inputs/IA_Fire`
  (params (ActionValue :type Boolean) (ElapsedSeconds :type "Float (double-precision)") (TriggeredSeconds :type "Float (double-precision)") (InputAction :type "InputAction Object Reference" :default "/Game/Cult_Custom/Characters/Police/Inputs/IA_Fire.IA_Fire")))

(event `Key|LeftMouseButton`
  (params (Key :type "Key Structure")))

(event `InputAction|Sprint`
  (params (Key :type "Key Structure")))

(event `InputAction|Sprint`
  (params (Key :type "Key Structure")))

(fn `GetCharacterMovement`
  (returns (ReturnValue :type "CharacterMovementComponent Object Reference"))
  (return (`self.CharacterMovement`)))

(fn `GetIsAiming`
  (returns (ReturnValue :type Boolean))
  (return (`self.IsAiming`)))

(fn `GetIsAttacking`
  (returns (ReturnValue :type Boolean))
  (return false))

(fn `GetIsPakour`
  (returns (ReturnValue :type Boolean))
  (return false))

(fn `GetIsPerforming`
  (returns (ReturnValue :type Boolean))
  (return false))

(fn `GetIsShooting`
  (returns (ReturnValue :type Boolean))
  (return false))

(fn `GetMesh`
  (returns (ReturnValue :type "SkeletalMeshComponent Object Reference"))
  (return (`self.Mesh`)))

(fn `GetMontageLength`
  (params (Input :type "AnimMontage Object Reference"))
  (returns (ReturnValue :type "Float (double-precision)"))
  (return 0.0))

(fn `GetMotionWarping`
  (returns (ReturnValue :type "MotionWarpingComponent Object Reference"))
  (return null))

(fn `GetNearEnoughToPakour`
  (returns (ReturnValue :type Boolean))
  (return false))

(fn `GetPlayerCapsule`
  (returns (ReturnValue :type "CapsuleComponent Object Reference"))
  (return (`self.CapsuleComponent`)))

(fn `GetVaultType`
  (returns (ReturnValue :type Byte))
  (return 0))

(fn `GetWeaponType`
  (returns (ReturnValue :type "EWeaponType Enum"))
  (return (`self.CurrentWeapon`)))

(fn `UserConstructionScript`)