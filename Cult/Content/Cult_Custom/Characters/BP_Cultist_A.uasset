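; Cultist player character with vault parkour, bone hit reactions and healing input.
; Jump runs line traces for wall height and thickness, then vaults low walls using temporary Flying mode, disabled capsule collision and a montage.
; Hits start a blend-weight timeline and delayed bone impulse, though the physics-blend application is disconnected.
; H sends a heal request, movement cancels healing; older parkour and heal logic sits unwired, and ParkourComponent is only initialized.
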(event `InputAction|Jump`
  (params (Key :type "Key Structure"))
  (:`Pressed`
    (`self.Parkour`)))

(event `Key|SpaceBar`
  (params (Key :type "Key Structure"))
  ;[1 1 1] Detect Wall
)

(event `Key|R`
  (params (Key :type "Key Structure"))
  ;[1 1 1] Detect Wall
)

(event `self.ReceiveBeginPlay`
  (message `/ParkourSystem/Interfaces/Parkour_Interface.Set Initialize Referrence` (`self.ParkourComponent`) self (`self.SpringArm`) (`self.MotionWarping`) (`self.Camera`)))

(event `self.ReceiveAnyDamage`
  (params (Damage :type "Float (single-precision)") (DamageType :type "DamageType Object Reference") (InstigatedBy :type "Controller Object Reference") (DamageCauser :type "Actor Object Reference")))

(event `/Game/Cult_Custom/Characters/Interfaces/BPI_Player.BPI_HitReaction`
  (params (BoneName :type Name))
  (`KismetSystemLibrary.PrintString` "calledHitReaction")
  (if (!= BoneName "pelvis")
    (set `self.Bone Name` BoneName)
    (if (not (`self.BPI_IsHit`))
      (set `self.BPI_IsHit` true)
      (`|ExecutionSequence`
        (:`then_0`
          (bind (_direction _blendweight) (`Timeline|타임라인` :!via `PlayFromStart`)
            (:`Update`
              (set `self.Blend Weight` _blendweight))
            (:`Finished`
              (`SkeletalMeshComponent.SetAllBodiesPhysicsBlendWeight` (`self.Mesh`) 0.0 false)
              (`SkeletalMeshComponent.SetAllBodiesSimulatePhysics` (`self.Mesh`) false)
              (set `self.BPI_IsHit` false))))
        (:`then_1`
          (`KismetSystemLibrary.Delay` 0.048)
          (`PrimitiveComponent.AddImpulse` (`self.Mesh`) (* (`self.GetActorForwardVector` (`GameplayStatics.GetPlayerCameraManager` 0)) 10000.0) (`self.Bone Name`) true))))))

(event `Key|H`
  (params (Key :type "Key Structure"))
  (:`Pressed`
    (`self.SendTryHeal`)))

(event `self.ReceiveTick`
  (params (DeltaSeconds :type "Float (single-precision)"))
  (if (and (or (`self.ABP_DoHeal`) (`self.ABP_GetHeal`)) (> (`KismetMathLibrary.VSize` (`self.GetVelocity`)) 0.0))
    (set `self.ABP_DoHeal` false)
    (set `self.ABP_GetHeal` false)
    (`self.SendEndHeal`)))

(fn `Calculate Wall Height`
  (bind _returnvalue (+ (+ (`self.Wall Location`) (* (`KismetMathLibrary.GetForwardVector` (`KismetMathLibrary.MakeRotFromX` (`self.Wall Normal`))) -10.0)) (0.0 0.0 900.0)))
  (bind _outhit (`KismetSystemLibrary.LineTraceSingleForObjects` :`Start` _returnvalue :`End` (- _returnvalue (0.0 0.0 900.0)) :`ObjectTypes` (`self.Object Types`) :`DrawDebugType` (`self.Draw Debug Type`) :`TraceColor` (struct :`G` 1.0 :`B` 0.003697 :`A` 1.0) :`TraceHitColor` (struct :`R` 1.0 :`G` 0.897106 :`A` 1.0)))
  (set `self.Wall Height` (`.Location` (`GameplayStatics.BreakHitResult` _outhit)))
  (return))

(fn `Calculate Wall Tickness`
  (returns (ReturnValue :type Boolean) (Location :type "Vector Structure"))
  (bind _returnvalue (+ (+ (`self.Wall Location`) (* (`KismetMathLibrary.GetForwardVector` (`KismetMathLibrary.MakeRotFromX` (`self.Wall Normal`))) -50.0)) (0.0 0.0 900.0)))
  (bind (_outhit _returnvalue_2) (`KismetSystemLibrary.LineTraceSingleForObjects` :`Start` _returnvalue :`End` (- _returnvalue (0.0 0.0 900.0)) :`ObjectTypes` (`self.Object Types`) :`DrawDebugType` (`self.Draw Debug Type`) :`TraceColor` (struct :`G` 1.0 :`B` 0.003697 :`A` 1.0) :`TraceHitColor` (struct :`R` 1.0 :`G` 0.897106 :`A` 1.0)))
  (return _returnvalue_2 (`.Location` (`GameplayStatics.BreakHitResult` _outhit))))

(fn `Disable Input`
  (`CharacterMovementComponent.SetMovementMode` (`self.CharacterMovement`) "MOVE_Flying" 0)
  (`PrimitiveComponent.SetCollisionEnabled` (`self.CapsuleComponent`) "NoCollision"))

(fn `Enable Input`
  (`CharacterMovementComponent.SetMovementMode` (`self.CharacterMovement`) "MOVE_Falling" 0)
  (`PrimitiveComponent.SetCollisionEnabled` (`self.CapsuleComponent`) "QueryAndPhysics"))

(fn `GetCharacterMovement`
  (returns (ReturnValue :type "CharacterMovementComponent Object Reference"))
  (return null))

(fn `GetIsAiming`
  (returns (ReturnValue :type Boolean))
  (return false))

(fn `GetIsAttacking`
  (returns (ReturnValue :type Boolean))
  (return false))

(fn `GetIsHitByAnAttack`
  (returns (ReturnValue :type Boolean))
  (return (`self.bIsHitByAnAttack`)))

(fn `GetIsPakour`
  (returns (ReturnValue :type Boolean))
  (return false))

(fn `GetIsPerforming`
  (returns (ReturnValue :type Boolean))
  (return (`self.bIsPerformingRitual`)))

(fn `GetIsShooting`
  (returns (ReturnValue :type Boolean))
  (return false))

(fn `GetIsStunned`
  (returns (ReturnValue :type Boolean))
  (return (`self.bIsStunned`)))

(fn `GetMesh`
  (returns (ReturnValue :type "SkeletalMeshComponent Object Reference"))
  (return null))

(fn `GetMontageLength`
  (params (Input :type "AnimMontage Object Reference"))
  (returns (ReturnValue :type "Float (double-precision)"))
  (return 0.0))

(fn `GetMotionWarping`
  (returns (ReturnValue :type "MotionWarpingComponent Object Reference"))
  (return null))

(fn `GetNearEnoughToPakour`
  (returns (ReturnValue :type Boolean))
  (return false))

(fn `GetPlayerCapsule`
  (returns (ReturnValue :type "CapsuleComponent Object Reference"))
  (return null))

(fn `GetVaultType`
  (returns (ReturnValue :type Byte))
  (return 0))

(fn `GetWeaponType`
  (returns (ReturnValue :type "EWeaponType Enum"))
  (return "Baton"))

(fn `JumpHelperFunction`
  (bind (_returnvalue_x _returnvalue_y _returnvalue_z) (`KismetMathLibrary.BreakVector` (`self.K2_GetActorLocation`)))
  (if (`self.JumpHelper`)
    (`self.K2_SetActorLocation` (`KismetMathLibrary.MakeVector` _returnvalue_x _returnvalue_y (`KismetMathLibrary.FInterpTo` _returnvalue_z (+ _returnvalue_z (`self.WallHeight2`)) (`GameplayStatics.GetWorldDeltaSeconds`) 4.0)))))

(fn `UserConstructionScript`)