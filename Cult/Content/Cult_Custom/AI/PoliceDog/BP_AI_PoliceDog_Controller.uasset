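; AI controller for the police dog, driving its behavior tree and blackboard.
; Five seconds after possession it runs the tree, stores the first Police-tagged actor as Master and sets an initial dog AI state.
; When perception senses a Cultist-tagged actor, it stores it as TargetPlayer and switches state to start chasing.
; Losing that actor clears TargetPlayer but leaves the state unchanged.
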(event `self.ReceivePossess`
  (params (PossessedPawn :type "Pawn Object Reference"))
  (`KismetSystemLibrary.Delay` 5.0)
  (`self.RunBehaviorTree` "/Game/Cult_Custom/AI/PoliceDog/BT_PoliceDog.BT_PoliceDog")
  (bind _blackboardcomponent (`self.UseBlackboard` "/Game/Cult_Custom/AI/PoliceDog/BB_PoliceDog.BB_PoliceDog"))
  (bind _outactors (`GameplayStatics.GetAllActorsWithTag` "Police"))
  (`BlackboardComponent.SetValueAsObject` _blackboardcomponent "Master" (`|GetArrayItem` _outactors))
  (`BlackboardComponent.SetValueAsEnum` _blackboardcomponent "AIState" (enumliteral `/Game/Cult_Custom/AI/PoliceDog/E_DogAIState` "NewEnumerator0")))

(event `self.AIPerception.OnTargetPerceptionUpdated`
  (params (Actor :type "Actor Object Reference") (Stimulus :type "AIStimulus Structure"))
  (bind _blackboard (`self.Blackboard`))
  (if (`self.ActorHasTag` Actor "Cultist")
    (if (`.bSuccessfullySensed` (break `AIStimulus` Stimulus))
      (`BlackboardComponent.SetValueAsObject` _blackboard "TargetPlayer" Actor)
      (`BlackboardComponent.SetValueAsEnum` _blackboard "AIState" (enumliteral `/Game/Cult_Custom/AI/PoliceDog/E_DogAIState` "NewEnumerator3"))
      (`KismetSystemLibrary.PrintString` "StartChasing")
      (else
        (`BlackboardComponent.SetValueAsObject` (`self.Blackboard`) "TargetPlayer" null)))))

(fn `UserConstructionScript`)