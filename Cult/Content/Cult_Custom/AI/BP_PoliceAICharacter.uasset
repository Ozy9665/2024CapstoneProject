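; Police AI character Blueprint that exposes a set of state and component getters, apparently for a shared character interface.
; Only the attacking and weapon type getters return live data, from IsAttacking and CurrentWeapon.
; Aiming, shooting, performing, parkour, vault and montage getters return false or zero, and component getters return nothing.
; The event graph and construction script contain no logic.
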(fn `GetCharacterMovement`
  (returns (ReturnValue :type "CharacterMovementComponent Object Reference"))
  (return null))

(fn `GetIsAiming`
  (returns (ReturnValue :type Boolean))
  (return false))

(fn `GetIsAttacking`
  (returns (ReturnValue :type Boolean))
  (return (`self.bIsAttacking`)))

(fn `GetIsPakour`
  (returns (ReturnValue :type Boolean))
  (return false))

(fn `GetIsPerforming`
  (returns (ReturnValue :type Boolean))
  (return false))

(fn `GetIsShooting`
  (returns (ReturnValue :type Boolean))
  (return false))

(fn `GetMesh`
  (returns (ReturnValue :type "SkeletalMeshComponent Object Reference"))
  (return null))

(fn `GetMontageLength`
  (params (Input :type "AnimMontage Object Reference"))
  (returns (ReturnValue :type "Float (double-precision)"))
  (return 0.0))

(fn `GetMotionWarping`
  (returns (ReturnValue :type "MotionWarpingComponent Object Reference"))
  (return null))

(fn `GetNearEnoughToPakour`
  (returns (ReturnValue :type Boolean))
  (return false))

(fn `GetPlayerCapsule`
  (returns (ReturnValue :type "CapsuleComponent Object Reference"))
  (return null))

(fn `GetVaultType`
  (returns (ReturnValue :type Byte))
  (return 0))

(fn `GetWeaponType`
  (returns (ReturnValue :type "EWeaponType Enum"))
  (return (`self.CurrentWeapon`)))

(fn `UserConstructionScript`)