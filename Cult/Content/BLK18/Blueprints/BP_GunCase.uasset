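; BP_GunCase is a gun case prop with a hinged lid, buckle and handle, each posed from a 0 to 1 value.
; UpdateCasePose lerps those values into relative roll rotations, and the construction script calls it to apply the configured pose.
; QuickOpen steps through closed, partly open and fully open presets with a looping MultiGate, then refreshes the pose.
; An OpenCase timeline for animated opening is present but never triggered.
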(event `QuickOpen`
  ;[0 0 0] QuickOpen
  (`|MultiGate` false true 1
    (:`Out 0`
      (set `self.BuckleOpenClose` 0.0)
      (set `self.LidOpenClose` 0.0))
    (:`Out 1`
      (set `self.BuckleOpenClose` 1.0)
      (set `self.LidOpenClose` 0.5))
    (:`Out 2`
      (set `self.BuckleOpenClose` 1.0)
      (set `self.LidOpenClose` 0.75))
    (:`Out 3`
      (set `self.BuckleOpenClose` 1.0)
      (set `self.LidOpenClose` 1.0)))
  (`self.UpdateCasePose`))

(fn `UpdateCasePose`
  ;[0 0 0] Case Pose
  ;;[1 1 1] Lid Open Close
  (`SceneComponent.K2_SetRelativeRotation` (`self.Lid`) (`KismetMathLibrary.MakeRotator` (`KismetMathLibrary.Lerp` 0.0 -180.0 (`self.LidOpenClose`))) false false)
  ;;[1 1 1] Buckle Open Close
  (`SceneComponent.K2_SetRelativeRotation` (`self.Buckle_M`) (`KismetMathLibrary.MakeRotator` (`KismetMathLibrary.Lerp` 0.0 -180.0 (`self.BuckleOpenClose`))) false false)
  ;;[1 1 1] Handle Rotation
  (`SceneComponent.K2_SetRelativeRotation` (`self.Handle`) (`KismetMathLibrary.MakeRotator` (`KismetMathLibrary.Lerp` 0.0 -180.0 (`self.HandleRotation`))) false false))

(fn `UserConstructionScript`
  (`self.UpdateCasePose`))